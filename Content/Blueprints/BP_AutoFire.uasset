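; BP_AutoFire is an actor that automatically fires projectiles for as long as it is in play.
; On BeginPlay it starts a looping short-interval timer bound to its Fire event.
; Each Fire spawns a BP_Projectile at the actor's own transform, so shots inherit its location and orientation.
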(event Custom|Fire
  (Game|SpawnActorfromClass "/Game/Blueprints/Weapon/Projectiles/BP_Projectile.BP_Projectile_C" (Transformation|GetActorTransform self) "Undefined" "MultiplyWithRoot" 0 0))

(event EventBeginPlay
  (|CallParentFunction)
  (Utilities|Time|SetTimerbyEvent (delegate Custom|Fire) 0.2 true))

(event Collision|EventActorBeginOverlap
  (params (OtherActor :type Actor%20Object%20Reference))
  (|CallParentFunction OtherActor) ; This node is disabled and will not be called.\nDrag off pins to build functionality.
)

(event EventTick
  (params (DeltaSeconds :type Float%20%28single-precision%29))
  (|CallParentFunction DeltaSeconds) ; This node is disabled and will not be called.\nDrag off pins to build functionality.
)

(fn ConstructionScript
  (|CallParentFunction))