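; BP_SCharacter3 is a character Blueprint that opens and closes the in-game menu from the 1 and Escape keys.
; Both keys share one toggle driven by the IsMenuOpen flag.
; Opening creates a new WBP_InGameMenu widget, adds it to the viewport, and switches player 0 to game-and-UI input with a visible cursor.
; Closing removes the widget, restores game-only input and hides the cursor.
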(event Input|KeyboardEvents|Escape
  (params (Key :type Key%20Structure))
  (bind _returnvalue (Game|GetPlayerController 0))
  (:Pressed
    (if (not (Variables|Default|GetIsMenuOpen))
      (Variables|Default|SetIsMenuOpen true)
      (bind _returnvalue_2 (UserInterface|CreateWidget "/Game/Blueprints/HUD/WBP_InGameMenu.WBP_InGameMenu_C"))
      (UserInterface|Viewport|AddtoViewport _returnvalue_2 0)
      (Input|SetInputModeGameandUI _returnvalue 0 "DoNotLock" true false)
      (Variables|/Script/Engine.PlayerController|SetbShowMouseCursor _returnvalue true)
      (else
        (Variables|Default|SetIsMenuOpen false)
        (Widget|RemovefromParent _returnvalue_2)
        (Input|SetInputModeGameOnly _returnvalue false)
        (Variables|/Script/Engine.PlayerController|SetbShowMouseCursor _returnvalue false)))))

(event Input|KeyboardEvents|1
  (params (Key :type Key%20Structure))
  (bind _returnvalue (Game|GetPlayerController 0))
  (:Pressed
    (if (not (Variables|Default|GetIsMenuOpen))
      (Variables|Default|SetIsMenuOpen true)
      (bind _returnvalue_2 (UserInterface|CreateWidget "/Game/Blueprints/HUD/WBP_InGameMenu.WBP_InGameMenu_C"))
      (UserInterface|Viewport|AddtoViewport _returnvalue_2 0)
      (Input|SetInputModeGameandUI _returnvalue 0 "DoNotLock" true false)
      (Variables|/Script/Engine.PlayerController|SetbShowMouseCursor _returnvalue true)
      (else
        (Variables|Default|SetIsMenuOpen false)
        (Widget|RemovefromParent _returnvalue_2)
        (Input|SetInputModeGameOnly _returnvalue false)
        (Variables|/Script/Engine.PlayerController|SetbShowMouseCursor _returnvalue false)))))

(fn ConstructionScript)